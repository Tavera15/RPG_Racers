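; AI-driven car NPC that loops through a list of checkpoints.
; Tick reissues MoveToActor on the current checkpoint, advancing and wrapping the index on arrival, and damage is forwarded to PlayerStats.
; Overlapping MyCar_BP zeroes that car's velocity and stops this AI's movement until the next Tick move request.
; A timer-repeated move to Store_A_BP has no caller here, and inventory-add nodes are disconnected.
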(event `self.ReceiveBeginPlay`)

(event `MyMoveToActor`
  (bind _asmy_aicontroller (cast `/Game/NPC/MyAIController` (`AIBlueprintHelperLibrary.GetAIController` self)))
  (bind _outactors (`GameplayStatics.GetAllActorsOfClass` "/Game/Blueprints/Store_A_BP.Store_A_BP_C"))
  (`AIController.MoveToActor` _asmy_aicontroller (`|GetArrayItem` _outactors) 100.0 false true true null true)
  (`KismetSystemLibrary.K2_SetTimerDelegate` (delegate `MyMoveToActor`) 0.1 true))

(event `self.ReceiveTick`
  (params (DeltaSeconds :type "Float (single-precision)"))
  (bind _returnvalue (+ (`self.IndexToGo`) 1))
  (bind _returnvalue_2 (`AIController.MoveToActor` (`AIBlueprintHelperLibrary.GetAIController` self) (`|GetArrayItem` (`self.Checkpoints`) (`self.IndexToGo`)) -1.0 false true true null true))
  (if (`|EnumEquality` _returnvalue_2 "AlreadyAtGoal")
    (if (== _returnvalue (`KismetArrayLibrary.Array_Length` (`self.Checkpoints`)))
      (set `self.IndexToGo` 0)
      (else
        (set `self.IndexToGo` _returnvalue)))))

(event `self.ReceiveAnyDamage`
  (params (Damage :type "Float (single-precision)") (DamageType :type "DamageType Object Reference") (InstigatedBy :type "Controller Object Reference") (DamageCauser :type "Actor Object Reference"))
  (`PlayerStats_AC.ReceiveDamage` (`self.PlayerStats`) Damage))

(event `self.ReceiveActorBeginOverlap`
  (params (OtherActor :type "Actor Object Reference"))
  (bind _asmy_car_bp (cast `/Game/Blueprints/MyCar_BP` OtherActor))
  (set `MovementComponent.Velocity` (0.0 0.0 0.0) (`self.GetComponentByClass` _asmy_car_bp "/Script/RPG_Racers.CarMovementComponent"))
  (`Controller.StopMovement` (`AIBlueprintHelperLibrary.GetAIController` self)))

(fn `UserConstructionScript`)