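; Yellow is a player car Blueprint that handles race start, damage with respawn, and pausing.
; On BeginPlay it calls OpenStore after a short delay and again after the checkpoint start delay, then locks inventory and saves starting driving force to PlayerStats.
; Damage routes through PlayerStats; a true result stops the car, briefly spawns fire, then respawns.
; Q shows the PauseScreen widget and cursor and pauses the game.
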(event `Key|Q`
  (params (Key :type "Key Structure"))
  (bind _returnvalue (`GameplayStatics.GetPlayerController` 0))
  (:`Pressed`
    (bind _returnvalue_2 (`|CreateWidget` "/Game/HUDs/PauseScreen.PauseScreen_C" _returnvalue))
    (bind _output_get (set `self.PauseScreen` _returnvalue_2))
    (set `PlayerController.bShowMouseCursor` true _returnvalue)
    (`UserWidget.AddToViewport` _output_get 0)
    (`GameplayStatics.SetGamePaused` true)))

(event `self.ReceiveBeginPlay`
  (`KismetSystemLibrary.Delay` 1.0)
  (`self.OpenStore`)
  (`KismetSystemLibrary.Delay` (`PlayerCheckpoints_A.timeToStart` (`PlayerStats_AC.LevelCheckpoints` (`self.PlayerStats`))))
  (`self.OpenStore`)
  (set `InventoryComponent.canAccessInventory` false (`self.InventoryComponent`))
  (set `PlayerStats_AC.StartingMaxDrivingForce` (`CarMovementComponent.MaxDrivingForce` (`self.CarMovementComp`)) (`self.PlayerStats`)))

(event `self.ReceiveActorBeginOverlap`
  (params (OtherActor :type "Actor Object Reference")))

(event `self.ReceiveAnyDamage`
  (params (Damage :type "Float (single-precision)") (DamageType :type "DamageType Object Reference") (InstigatedBy :type "Controller Object Reference") (DamageCauser :type "Actor Object Reference"))
  (bind (_returnvalue_location _returnvalue_rotation) (`KismetMathLibrary.BreakTransform` (`self.GetTransform`)))
  (bind _returnvalue (`PlayerStats_AC.ReceiveDamage` (`self.PlayerStats`) Damage))
  (if _returnvalue
    (set `MovementComponent.Velocity` (0.0 0.0 0.0) (`self.CarMovementComp`))
    (bind _returnvalue_2 (`GameplayStatics.SpawnEmitterAtLocation` "/Game/StarterContent/Particles/P_Fire.P_Fire" (+ _returnvalue_location (0.0 0.0 50.0)) _returnvalue_rotation (2.0 2.0 2.0)))
    (`KismetSystemLibrary.Delay` 1.5)
    (`ActorComponent.K2_DestroyComponent` _returnvalue_2)
    (`PlayerStats_AC.Respawn` (`self.PlayerStats`))))

(event `self.ReceiveTick`
  (params (DeltaSeconds :type "Float (single-precision)")))

(fn `UserConstructionScript`)