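; BP_Checkpoint_A is an indexed checkpoint that reports to an actor's PlayerStats_AC and lights up when it is the next target.
; BeginPlay sizes its sphere from AcceptanceRadius and caches the first Yellow actor as the player.
; Overlapping actors with PlayerStats_AC get UpdateCheckpoint called with this Index.
; Tick polls the player's CheckpointToGo, showing the SpotLight only when it matches Index.
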(event `self.ReceiveBeginPlay`
  (bind _outactors (`GameplayStatics.GetAllActorsOfClass` "/Game/Blueprints/Yellow.Yellow_C"))
  (set `self.Player` (`|GetArrayItem` _outactors))
  (`SphereComponent.SetSphereRadius` (`self.Sphere`) (`self.AcceptanceRadius`) true))

(event `self.ReceiveActorBeginOverlap`
  (params (OtherActor :type "Actor Object Reference"))
  (bind _returnvalue (`self.GetComponentByClass` OtherActor "/Script/RPG_Racers.PlayerStats_AC"))
  (if (!= _returnvalue null)
    (`PlayerStats_AC.UpdateCheckpoint` _returnvalue (`self.Index`))))

(event `self.ReceiveTick`
  (params (DeltaSeconds :type "Float (single-precision)"))
  (bind _player (`self.Player`))
  (bind _spotlight (`self.SpotLight`))
  (if (!= _player null)
    (if (== (`self.Index`) (`PlayerStats_AC.CheckpointToGo` (`self.GetComponentByClass` _player "/Script/RPG_Racers.PlayerStats_AC")))
      (`SceneComponent.SetVisibility` _spotlight true false)
      (else
        (`SceneComponent.SetVisibility` _spotlight false false)))))

(fn `UserConstructionScript`)