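; Weapon pickup box that gives a random offensive weapon to a Yellow or IndCarAi actor that overlaps it.
; On BeginPlay it picks one of the OffensiveWeapon_Item_A_BP actors already in the level.
; On overlap it assigns that weapon if the actor's OffensiveWeapon check passes, then flags its owning ROW_Spawner_A as missing a box and destroys itself.
; Without a spawner owner it prints a debug string and remains.
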(event `self.ReceiveBeginPlay`
  (bind _outactors (`GameplayStatics.GetAllActorsOfClass` "/Game/Items/Offensive-Weapons/Bases/OffensiveWeapon_Item_A_BP.OffensiveWeapon_Item_A_BP_C"))
  (bind _output_get (set `self.AllWeapons` _outactors))
  (set `self.ROW` (`|GetArrayItem` _output_get (`KismetMathLibrary.RandomInteger` (`KismetArrayLibrary.Array_Length` _output_get)))))

(event `self.ReceiveActorBeginOverlap`
  (params (OtherActor :type "Actor Object Reference"))
  (bind _asyellow (cast `/Game/Blueprints/Yellow` OtherActor)
    (:`then`
      (if (== (`CarPawn.OffensiveWeapon` _asyellow) null)
        (set `CarPawn.OffensiveWeapon` (`self.ROW`) _asyellow)
        (bind _asrow_spawner_a (cast `/Game/Blueprints/ROW_Spawner_A` (`self.GetOwner`) :!label _label)
          (:`then`
            (set `/Game/Blueprints/ROW_Spawner_A.isMissingBox` true _asrow_spawner_a)
            (`self.K2_DestroyActor`))
          (:`CastFailed`
            (`KismetSystemLibrary.PrintString` "Hello")))))
    (:`CastFailed`
      (bind _asind_car_ai (cast `/Game/NPC/NewFolder/IndCarAi` OtherActor))
      (if (== (`/Game/NPC/NewFolder/IndCarAi.OffensiveWeapon` _asind_car_ai) null)
        (set `/Game/NPC/NewFolder/IndCarAi.OffensiveWeapon` (`self.ROW`) _asind_car_ai)
        (goto _label)))))

(fn `UserConstructionScript`)