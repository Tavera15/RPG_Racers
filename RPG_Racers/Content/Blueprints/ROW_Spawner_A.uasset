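; Weapon box spawner actor that places a WeaponBox_A at its own location and rotation, at 2.5x scale, on BeginPlay.
; Tick polls IsMissingBox and, when true, waits through a short Delay, spawns a replacement box and clears the flag.
; Each box has the spawner as its Owner, and nothing in this Blueprint sets the flag to true.
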(event `self.ReceiveBeginPlay`
  (bind (_returnvalue_location _returnvalue_rotation) (`KismetMathLibrary.BreakTransform` (`self.GetTransform`)))
  (`|SpawnActorFromClass` :`Class` "/Game/Blueprints/WeaponBox_A.WeaponBox_A_C" :`SpawnTransform` (`KismetMathLibrary.MakeTransform` _returnvalue_location _returnvalue_rotation (2.5 2.5 2.5)) :`CollisionHandlingOverride` "Undefined" :`TransformScaleMethod` "OverrideRootScale" :`Owner` self :`ROW` null :`Instigator` null))

(event `self.ReceiveTick`
  (params (DeltaSeconds :type "Float (single-precision)"))
  (bind (_returnvalue_location _returnvalue_rotation) (`KismetMathLibrary.BreakTransform` (`self.GetTransform`)))
  (if (`self.isMissingBox`)
    (`KismetSystemLibrary.Delay` 3.0)
    (`|SpawnActorFromClass` :`Class` "/Game/Blueprints/WeaponBox_A.WeaponBox_A_C" :`SpawnTransform` (`KismetMathLibrary.MakeTransform` _returnvalue_location _returnvalue_rotation (2.5 2.5 2.5)) :`CollisionHandlingOverride` "Undefined" :`TransformScaleMethod` "OverrideRootScale" :`Owner` self :`ROW` null :`Instigator` null)
    (set `self.isMissingBox` false)))

(fn `UserConstructionScript`)