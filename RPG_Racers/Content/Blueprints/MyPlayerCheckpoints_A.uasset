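; MyPlayerCheckpoints_A manages the start and finish of a race, enabling racing and presenting the winner.
; BeginPlay clears the winner widget and sets CanRace after a TimeToStart delay.
; Tick polls IsWinnerFound, creates a Winner_HUD with the Winner's display name, shows the mouse cursor and switches input to Game and UI.
; The widget is added to the viewport on both branches of its IsInViewport check.
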(event `self.ReceiveBeginPlay`
  (set `self.WinnerWidget` null)
  (`KismetSystemLibrary.Delay` (`self.timeToStart`))
  (set `self.canRace` true))

(event `self.ReceiveTick`
  (params (DeltaSeconds :type "Float (single-precision)"))
  (bind _returnvalue (`GameplayStatics.GetPlayerController` 0))
  (if (and (== (`self.WinnerWidget`) null) (`self.isWinnerFound`))
    (bind _returnvalue_2 (`|CreateWidget` "/Game/HUDs/Winner_HUD.Winner_HUD_C" _returnvalue (`KismetTextLibrary.Conv_StringToText` (`KismetSystemLibrary.GetDisplayName` (`self.winner`)))))
    (bind _output_get (set `self.WinnerWidget` _returnvalue_2))
    (set `PlayerController.bShowMouseCursor` true _returnvalue)
    (`WidgetBlueprintLibrary.SetInputMode_GameAndUIEx` _returnvalue _output_get "DoNotLock" false)
    (if (`Widget.IsInViewport` _output_get)
      (bind _output_get_2 (set `self.WinnerWidget` _output_get))
      (`UserWidget.AddToViewport` _output_get_2 0)
      (else
        (`UserWidget.AddToViewport` _output_get 0)))))

(fn `UserConstructionScript`)